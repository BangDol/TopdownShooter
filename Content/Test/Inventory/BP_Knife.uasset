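; BP_Knife is a knife item actor for the test inventory system.
; It overrides GetDefaultItemObject to construct a BP_ItemObject holding its grid footprint, normal and rotated icon materials, and BP_Knife as the item class.
; Its event graph holds only disabled default events, and the construction script just calls the parent, so any other behavior comes from the parent class.
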(event EventBeginPlay
  (|CallParentFunction) ; 지금 이 노드는 비활성 상태입니다. \n핀을 끌어서 다른 노드를 연결하면 활성화됩니다.
)

(event Collision|EventActorBeginOverlap
  (params (OtherActor :type Actor%20Object%20Reference))
  (|CallParentFunction OtherActor) ; 지금 이 노드는 비활성 상태입니다. \n핀을 끌어서 다른 노드를 연결하면 활성화됩니다.
)

(event EventTick
  (params (DeltaSeconds :type Float%20%28single-precision%29))
  (|CallParentFunction DeltaSeconds) ; 지금 이 노드는 비활성 상태입니다. \n핀을 끌어서 다른 노드를 연결하면 활성화됩니다.
)

(fn ConstructionScript
  (|CallParentFunction))

(fn GetDefaultItemObject
  (bind _returnvalue (Game|ConstructObjectfromClass "/Game/Test/Inventory/BP_ItemObject.BP_ItemObject_C" self (Utilities|Struct|MakeIntPoint 1 2) "/Game/Assets/Interactable/Items/Icons/MI_Icon_Knife.MI_Icon_Knife" "/Game/Assets/Interactable/Items/Icons/MI_Icon_Knife_R.MI_Icon_Knife_R" "BP_Knife_C"))
  (return _returnvalue))