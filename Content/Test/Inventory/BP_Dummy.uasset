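; BP_Dummy is a test pickup actor that puts its ItemObject into the player's inventory on interaction.
; On BeginPlay it fills an invalid ItemObject from GetDefaultItemObject, whose body here is empty and returns no item.
; OnInteract casts player character 0 to BP_Player, calls TryAddItem on its inventory component, and destroys the actor only if the add succeeds.
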(event EventBeginPlay
  (if (not (Utilities|IsValid (Variables|Private|GetItemObject)))
    (bind _itemobject (Private|GetDefaultItemObject))
    (Variables|Private|SetItemObject _itemobject)))

(event EventOnInteract
  (bind _asbp_player (Utilities|Casting|CastToBP_Player (Game|GetPlayerCharacter 0)))
  (bind _added (Default|TryAddItem (Variables|/Game/Assets/Characters/Player/BP_Player.BP_Player_C|GetInventoryComponent1 _asbp_player) (Variables|Private|GetItemObject)))
  (if _added
    (Actor|DestroyActor)))

(fn ConstructionScript)

(fn GetDefaultItemObject
  (return 0))